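; LevelAnchor is a level actor that culls stray projectiles and enemies through two overlap volumes.
; Its Front volume destroys any overlapping ShotPlain or TensionBeam.
; Its BaddieKillbox volume destroys any overlapping Baddie, BaddieBob or BaddieWave, identifying each through a chain of casts and ignoring all other actors.
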(event OnComponentBeginOverlap(Front)
  (params (OtherActor :type Actor%20Object%20Reference) (OtherComp :type Primitive%20Component%20Object%20Reference) (OtherBodyIndex :type Integer) (bFromSweep :type Boolean) (SweepResult :type Hit%20Result%20Structure%20%28by%20ref%29))
  (bind _asshot_plain (Utilities|Casting|CastToShotPlain OtherActor)
    (:then
      (Actor|DestroyActor _asshot_plain))
    (:CastFailed
      (bind _astension_beam (Utilities|Casting|CastToTensionBeam OtherActor))
      (Actor|DestroyActor _astension_beam))))

(event OnComponentBeginOverlap(BaddieKillbox)
  (params (OtherActor :type Actor%20Object%20Reference) (OtherComp :type Primitive%20Component%20Object%20Reference) (OtherBodyIndex :type Integer) (bFromSweep :type Boolean) (SweepResult :type Hit%20Result%20Structure%20%28by%20ref%29))
  (bind _asbaddie (Utilities|Casting|CastToBaddie OtherActor)
    (:then
      (Actor|DestroyActor _asbaddie))
    (:CastFailed
      (bind _asbaddie_bob (Utilities|Casting|CastToBaddieBob OtherActor)
        (:then
          (Actor|DestroyActor _asbaddie_bob))
        (:CastFailed
          (bind _asbaddie_wave (Utilities|Casting|CastToBaddieWave OtherActor))
          (Actor|DestroyActor _asbaddie_wave))))))

(event EventBeginPlay)

(event EventActorBeginOverlap
  (params (OtherActor :type Actor%20Object%20Reference)))

(event EventTick
  (params (DeltaSeconds :type Float%20%28single-precision%29)))

(fn ConstructionScript)