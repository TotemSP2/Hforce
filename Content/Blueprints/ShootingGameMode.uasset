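; Game mode for a shooting game that owns the HUD, session stats and the game-over flow.
; BeginPlay shows the HUD and clears the Gamestart flag after a short delay.
; Until game over, Tick polls the ShootingCharacter to copy score, track the highest combo and mirror its boss-spawned state into Bossfight.
; The Dead event removes all widgets, then after delays shows the game-over widget and returns to the START level.
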(event Custom|Dead
  (Viewport|RemoveAllWidgets)
  (Utilities|FlowControl|Delay 3.0)
  (CallFunction|GameOver)
  (Utilities|FlowControl|Delay 3e+01)
  (Game|OpenLevel(byName) "START"))

(event EventBeginPlay
  (bind _returnvalue (UserInterface|CreateWidget "/Game/UMG/GAMEHUD.GAMEHUD_C"))
  (UserInterface|Viewport|AddtoViewport _returnvalue 0)
  (Utilities|FlowControl|Delay 1.5)
  (Variables|Default|SetGamestart false))

(event EventTick
  (params (DeltaSeconds :type Float%20%28single-precision%29))
  (if (not (Variables|Default|GetGameIsOver))
    (CallFunction|GetScore)
    (CallFunction|GetHighestCombo)
    (bind _asshooting_character (Utilities|Casting|CastToShootingCharacter (Game|GetPlayerCharacter 0)))
    (if (Variables|/Game/Blueprints/ShootingCharacter.ShootingCharacter_C|GetBossSpawned? _asshooting_character)
      (if (Variables|/Game/Blueprints/ShootingCharacter.ShootingCharacter_C|GetDebugMode _asshooting_character)
        (Development|PrintString "Bossfight"))
      (Variables|Default|SetBossfight true)
      (else
        (Variables|Default|SetBossfight false)))))

(fn ConstructionScript)

(fn GetScore
  (bind _asshooting_character (Utilities|Casting|CastToShootingCharacter (Game|GetPlayerCharacter 0)))
  (Variables|Default|SetGameScore (Variables|/Game/Blueprints/ShootingCharacter.ShootingCharacter_C|GetScore _asshooting_character)))

(fn GameOver
  (Variables|Default|SetGameIsOver true)
  (bind _returnvalue (UserInterface|CreateWidget "/Game/UMG/GAMEOVER.GAMEOVER_C"))
  (UserInterface|Viewport|AddtoViewport _returnvalue 0))

(fn GetHighestCombo
  (bind _asshooting_character (Utilities|Casting|CastToShootingCharacter (Game|GetPlayerCharacter 0)))
  (if (> (Variables|/Game/Blueprints/ShootingCharacter.ShootingCharacter_C|GetCombo _asshooting_character) (Variables|Default|GetHighCombo))
    (Variables|Default|SetHighCombo (Variables|/Game/Blueprints/ShootingCharacter.ShootingCharacter_C|GetCombo _asshooting_character))))