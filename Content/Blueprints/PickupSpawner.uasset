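; Pickup spawner for a shooter that periodically spawns one of two pickups, apparently TBeam and shield, at its PickupSpawn point.
; A SweepGameArea timeline offsets the actor and feeds a random Delay, after which SpawnBaddie re-calls itself to keep spawning.
; Tick holds it at a fixed Y offset from the player, and boss-fight flags on the game mode or character destroy it.
; U and J keys force-spawn each pickup with a debug print.
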(event Custom|SpawnBaddie
  (bind _asshooting_character (Utilities|Casting|CastToShootingCharacter (Game|GetPlayerCharacter 0)))
  (if (Variables|/Game/Blueprints/ShootingCharacter.ShootingCharacter_C|GetBossSpawned? _asshooting_character)
    (Actor|DestroyActor)
    (else
      (Utilities|FlowControl|Delay (Math|Random|RandomFloatinRange 7.5 11.0))
      (Game|SpawnActorfromClass (Utilities|Array|Get(acopy) (Variables|Default|GetPickups) (Math|Random|RandomIntegerinRange 0 1)) (Transformation|GetWorldTransform (Variables|Default|GetPickupSpawn)) "Undefined" 0 0)
      (CallFunction|SpawnBaddie))))

(event EventBeginPlay
  (bind _height (Timeline|SweepGameArea Play)
    (:Update
      (Transformation|AddActorLocalOffset _height true false)
      (Utilities|FlowControl|Delay (Math|Random|RandomFloatinRange 7.5 11.0))
      (Game|SpawnActorfromClass (Utilities|Array|Get(acopy) (Variables|Default|GetPickups) (Math|Random|RandomIntegerinRange 0 1)) (Transformation|GetWorldTransform (Variables|Default|GetPickupSpawn)) "Undefined" 0 0)
      (CallFunction|SpawnBaddie))))

(event EventTick
  (params (DeltaSeconds :type Float%20%28single-precision%29))
  (bind _returnvalue (Transformation|GetActorLocation))
  (bind (_x _y _z) (Math|Vector|BreakVector _returnvalue))
  ;[1 1 1] Position
  (bind _asshooting_game_mode (Utilities|Casting|CastToShootingGameMode (Game|GetGameMode)))
  (if (Variables|/Game/Blueprints/ShootingGameMode.ShootingGameMode_C|GetBossfight _asshooting_game_mode)
    (Actor|DestroyActor)
    (elif (Variables|/Game/Blueprints/ShootingGameMode.ShootingGameMode_C|GetBossfight _asshooting_game_mode)
      (Actor|DestroyActor)
      (else
        (Transformation|SetActorLocation (Math|Vector|MakeVector _x (+ (.Y (Math|Vector|BreakVector (Transformation|GetActorLocation (Game|GetPlayerCharacter 0)))) -4e+03) _z) false false)))))

(event Input|KeyboardEvents|U
  (params (Key :type Key%20Structure :default "AnyKey"))
  (:Pressed
    (Game|SpawnActorfromClass (Utilities|Array|Get(acopy) (Variables|Default|GetPickups)) (Transformation|GetWorldTransform (Variables|Default|GetPickupSpawn)) "Undefined" 0 0)
    (Development|PrintString "TBeam out")))

(event Input|KeyboardEvents|J
  (params (Key :type Key%20Structure :default "AnyKey"))
  (:Pressed
    (Game|SpawnActorfromClass (Utilities|Array|Get(acopy) (Variables|Default|GetPickups) 1) (Transformation|GetWorldTransform (Variables|Default|GetPickupSpawn)) "Undefined" 0 0)
    (Development|PrintString "shield out")))

(fn ConstructionScript)

(fn ListofBaddies
  (Variables|Default|SetBaddieList (Utilities|Array|MakeArray "/Game/Blueprints/Baddie.Baddie_C" "/Game/Blueprints/BaddieBob.BaddieBob_C")))