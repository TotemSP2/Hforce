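; BaddieBoss is a boss enemy that fires from three guns, launches random minions from four flight decks and destroys itself when Health runs out.
; Endless Delay loops started on BeginPlay drive shooting, spawning and a scripted ProjectileMovement velocity pattern.
; Sphere overlap drops the player's shield or, if already down, kills them.
; Destruction flags the boss dead, plays death effects and removes all widgets; stay-on-screen logic is unwired.
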(event OnComponentBeginOverlap(Sphere)
  (params (OtherActor :type Actor%20Object%20Reference) (OtherComp :type Primitive%20Component%20Object%20Reference) (OtherBodyIndex :type Integer) (bFromSweep :type Boolean) (SweepResult :type Hit%20Result%20Structure%20%28by%20ref%29))
  (bind _asshooting_character (Utilities|Casting|CastToShootingCharacter OtherActor))
  (if (Variables|/Game/Blueprints/ShootingCharacter.ShootingCharacter_C|GetIsShieldDown _asshooting_character)
    (if (not (Variables|/Game/Blueprints/ShootingCharacter.ShootingCharacter_C|GetIsDead _asshooting_character))
      (Default|Dead _asshooting_character)
      (bind _asshooting_game_mode (Utilities|Casting|CastToShootingGameMode (Game|GetGameMode)))
      (Default|Dead _asshooting_game_mode))
    (else
      (Variables|/Game/Blueprints/ShootingCharacter.ShootingCharacter_C|SetIsShieldDown _asshooting_character true))))

(event Custom|Begin%20Movement
  (Variables|/Script/Engine.MovementComponent|SetVelocity (Variables|Default|GetProjectileMovement) "0.000000,500.000000, 0" :!label _label)
  (Utilities|FlowControl|Delay 2.0)
  (Variables|/Script/Engine.MovementComponent|SetVelocity (Variables|Default|GetProjectileMovement) "0.000000,0.000000,500.000000")
  (Utilities|FlowControl|Delay 1.0)
  (Variables|/Script/Engine.MovementComponent|SetVelocity (Variables|Default|GetProjectileMovement) "0.000000,250.000000,-750.000000")
  (Utilities|FlowControl|Delay 1.0)
  (Variables|/Script/Engine.MovementComponent|SetVelocity (Variables|Default|GetProjectileMovement) "0.000000,1700.000000,0.000000")
  (Utilities|FlowControl|Delay 0.2)
  (Variables|/Script/Engine.MovementComponent|SetVelocity (Variables|Default|GetProjectileMovement) "0.000000,-1700.000000,250.000000")
  (Utilities|FlowControl|Delay 0.85)
  (goto _label))

(event Custom|BeginShooting
  (Game|SpawnActorfromClass "/Game/Blueprints/ShotBad.ShotBad_C" (Transformation|GetWorldTransform (Variables|Default|GetGun1)) "Undefined" 0 0 :!label _label)
  (Game|SpawnActorfromClass "/Game/Blueprints/ShotBad.ShotBad_C" (Transformation|GetWorldTransform (Variables|Default|GetGun2)) "Undefined" 0 0)
  (Game|SpawnActorfromClass "/Game/Blueprints/ShotBad.ShotBad_C" (Transformation|GetWorldTransform (Variables|Default|GetGun3)) "Undefined" 0 0)
  (Audio|PlaySoundatLocation "/Game/noise/Weapons/bossshot_Cue.bossshot_Cue" (Transformation|GetActorLocation))
  (Utilities|FlowControl|Delay 0.75)
  (goto _label))

(event EventTick
  (params (DeltaSeconds :type Float%20%28single-precision%29))
  (if (<= (Variables|Default|GetHealth) 0)
    (Actor|DestroyActor)))

(event EventBeginPlay
  (bind _returnvalue (Math|Random|RandomIntegerinRange 0 2))
  (bind _baddiesondeck (Variables|Default|GetBaddiesonDeck))
  (bind _item (Utilities|Array|Get(acopy) _baddiesondeck _returnvalue))
  (CallFunction|BeginMovement)
  (CallFunction|BeginShooting)
  (Game|SpawnActorfromClass _item (Transformation|GetWorldTransform (Variables|Default|GetFlightDeck1)) "Undefined" 0 0 :!label _label)
  (Game|SpawnActorfromClass _item (Transformation|GetWorldTransform (Variables|Default|GetFlightDeck2)) "Undefined" 0 0)
  (Game|SpawnActorfromClass _item (Transformation|GetWorldTransform (Variables|Default|GetFlightDeck3)) "Undefined" 0 0)
  (Game|SpawnActorfromClass _item (Transformation|GetWorldTransform (Variables|Default|GetFlightDeck4)) "Undefined" 0 0)
  (Utilities|FlowControl|Delay 2.0)
  (goto _label))

(event EventDestroyed
  (bind _returnvalue (Transformation|GetActorLocation))
  (bind _asshooting_character (Utilities|Casting|CastToShootingCharacter (Game|Player|GetPlayerPawn 0)))
  (Variables|/Game/Blueprints/ShootingCharacter.ShootingCharacter_C|SetisBossDead _asshooting_character true)
  (Game|SpawnActorfromClass "/Game/Blueprints/boss_death.boss_death_C" (Math|Conversions|ToTransform(Vector) _returnvalue) "Undefined" 0 0)
  (bind _returnvalue_2 (Effects|SpawnEmitteratLocation "/Game/PARTICLES/A_Bossdead.A_Bossdead" _returnvalue))
  (Transformation|SetRelativeScale3D _returnvalue_2 "5.000000,5.000000,5.000000")
  (Audio|PlaySound2D "/Game/noise/Impacts/Bossdead_Cue.Bossdead_Cue")
  (Viewport|RemoveAllWidgets))

(fn ConstructionScript)