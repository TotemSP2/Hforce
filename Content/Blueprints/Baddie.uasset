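; Baddie is a short-lived enemy actor that harms a ShootingCharacter on contact and destroys itself ten seconds after spawning.
; Its Sphere overlap casts the other actor to ShootingCharacter and checks the shield state.
; A raised shield is knocked down and the Baddie is destroyed, while a downed shield means the character dies, unless already dead.
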(event OnComponentBeginOverlap(Sphere)
  (params (OtherActor :type Actor%20Object%20Reference) (OtherComp :type Primitive%20Component%20Object%20Reference) (OtherBodyIndex :type Integer) (bFromSweep :type Boolean) (SweepResult :type Hit%20Result%20Structure%20%28by%20ref%29))
  (bind _asshooting_character (Utilities|Casting|CastToShootingCharacter OtherActor))
  (if (Variables|/Game/Blueprints/ShootingCharacter.ShootingCharacter_C|GetIsShieldDown _asshooting_character)
    (if (not (Variables|/Game/Blueprints/ShootingCharacter.ShootingCharacter_C|GetIsDead _asshooting_character))
      (Default|Dead _asshooting_character))
    (else
      (Actor|DestroyActor)
      (Variables|/Game/Blueprints/ShootingCharacter.ShootingCharacter_C|SetIsShieldDown _asshooting_character true))))

(event EventBeginPlay
  (Utilities|FlowControl|Delay 1e+01)
  (Actor|DestroyActor))

(event Collision|EventActorBeginOverlap
  (params (OtherActor :type Actor%20Object%20Reference)))

(event EventTick
  (params (DeltaSeconds :type Float%20%28single-precision%29)))

(fn ConstructionScript)